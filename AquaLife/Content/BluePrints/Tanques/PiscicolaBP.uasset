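; Fish-farm tank actor (piscícola) whose trigger box lets the player enter its build puzzle and shows interaction prompts.
; BeginPlay swaps the Paper2D flipbook if this tank's puzzle is solved in the GameInstance array.
; Overlap records the tank index and picks prompt text from purchased-parts and disinfection flags, or opens one-time fish selection for solved tanks.
; End overlap clears entry permission and removes the prompt, then re-runs that same state check.
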(event OnComponentBeginOverlap(Box)
  (params (OverlappedComponent :type Primitive%20Component%20Object%20Reference) (OtherActor :type Actor%20Object%20Reference) (OtherComp :type Primitive%20Component%20Object%20Reference) (OtherBodyIndex :type Integer) (bFromSweep :type Boolean) (SweepResult :type Hit%20Result%20Structure%20%28by%20ref%29))
  (bind _returnvalue (Game|GetPlayerController 0))
  (bind _as_instancia (Variables|Default|GetAs%20Instancia))
  (bind _as_instancia_2 (Variables|Default|GetAs%20Instancia))
  (bind _refwidgetpiscicola (Variables|Default|GetRefWidGetPiscicola))
  (bind _as_instancia_3 (Variables|Default|GetAs%20Instancia))
  (bind _as_instancia_4 (Variables|Default|GetAs%20Instancia))
  (bind _partesblowercompradas (Variables|/Game/Instancia.Instancia_C|GetPartesBlowerCompradas _as_instancia_3))
  (bind _parteshidrobombacompradastodo (Variables|/Game/Instancia.Instancia_C|GetPartesHidroBombaCompradasTODO _as_instancia_3))
  (bind _textointeraccion (Variables|/Game/Interfaz/UI_PISCICOLA.UI_PISCICOLA_C|GetTextoInteraccion _refwidgetpiscicola))
  (bind _arraypiscicolas (Variables|/Game/Instancia.Instancia_C|GetArrayPiscicolas _as_instancia_4))
  ;[1 1 1] al entrar en contacto con el trigger
  (bind _asplayer_bp (Utilities|Casting|CastToPlayerBP OtherActor))
  (Variables|/Game/BluePrints/Personaje/PlayerBP.PlayerBP_C|SetpuedeEntrarPuzzle _asplayer_bp true)
  ;;[0.5677 0.8429 1] Muestra la UI al entrar
  (bind _returnvalue_2 (UserInterface|CreateWidget (Utilities|GetClass (Variables|Default|GetRefWidGetPiscicola))))
  (UserInterface|Viewport|AddtoViewport _returnvalue_2 0)
  (bind _output_get (Variables|/Game/Instancia.Instancia_C|SetIndiceActual _as_instancia_2 (Variables|Default|GetIndicePiscicola)))
  (if (.PuzzleResuelto (Utilities|Struct|BreakPiscicolaData (Utilities|Array|Get(acopy) (Variables|/Game/Instancia.Instancia_C|GetArrayPiscicolas _as_instancia_2) _output_get)))
    ;[0 0 0] Widget seleccion pez
    (if (.YaSeleccionoMojarra? (Utilities|Struct|BreakPiscicolaData (Utilities|Array|Get(acopy) (Variables|/Game/Instancia.Instancia_C|GetArrayPiscicolas _as_instancia) (Variables|/Game/Instancia.Instancia_C|GetIndiceActual _as_instancia))))
      ;[1 0 0] Cambios Andres
      (if (Variables|/Game/Instancia.Instancia_C|Getdesinfectado (Variables|Default|GetAs%20Instancia))
        ;[0 0 0] Lo que se muestra dependiendo de la condicion
        (Rendering|Components|TextRender|SetText _textointeraccion "Pulse X para interactuar con la piscicola")
        (else
          (Rendering|Components|TextRender|SetText (Variables|/Game/Interfaz/UI_PISCICOLA.UI_PISCICOLA_C|GetTextoInteraccion (Variables|Default|GetRefWidGetPiscicola)) "Antes de interactuar con los peces ve a desinfectarte")))
      (else
        (bind _returnvalue_3 (UserInterface|CreateWidget "/Game/Interfaz/UI_PECES.UI_PECES_C"))
        (bind _output_get_2 (Variables|Default|SetRefWidgetPeces _returnvalue_3))
        (UserInterface|Viewport|AddtoViewport _returnvalue_3 0)
        ;;[1 1 1] Mnaipular el mouse para seleccion
        (Variables|/Script/Engine.PlayerController|SetbShowMouseCursor _returnvalue true)
        (Input|SetInputModeUIOnly _returnvalue _output_get_2 "DoNotLock" false)
        (bind _structout (Utilities|Struct|SetmembersinPiscicolaData (Utilities|Array|Get(acopy) _arraypiscicolas (Variables|/Game/Instancia.Instancia_C|GetIndiceActual _as_instancia_4)) true))
        (Utilities|Array|SetArrayElem _arraypiscicolas (Variables|/Game/Instancia.Instancia_C|GetIndiceActual _as_instancia_4) _structout)))
    (elif (and _partesblowercompradas _parteshidrobombacompradastodo)
      (Rendering|Components|TextRender|SetText _textointeraccion "Pulse X para construir la piscicola")
      (elif _parteshidrobombacompradastodo
        (Rendering|Components|TextRender|SetText _textointeraccion "Hacen falta comprar las partes del blower. Ve a la tienda.")
        (elif _partesblowercompradas
          (Rendering|Components|TextRender|SetText _textointeraccion "Hacen falta comprar las partes de la hidrobomba. Ve a la tienda.")
          (else
            (Rendering|Components|TextRender|SetText _textointeraccion "Hace falta comprar las partes de la hidrobomba. Ve a la tienda.")))))))

(event OnComponentEndOverlap(Box)
  (params (OverlappedComponent :type Primitive%20Component%20Object%20Reference) (OtherActor :type Actor%20Object%20Reference) (OtherComp :type Primitive%20Component%20Object%20Reference) (OtherBodyIndex :type Integer))
  (bind _returnvalue (Game|GetPlayerController 0))
  (bind _as_instancia (Variables|Default|GetAs%20Instancia))
  (bind _refwidgetpiscicola (Variables|Default|GetRefWidGetPiscicola))
  (bind _as_instancia_2 (Variables|Default|GetAs%20Instancia))
  (bind _as_instancia_3 (Variables|Default|GetAs%20Instancia))
  (bind _partesblowercompradas (Variables|/Game/Instancia.Instancia_C|GetPartesBlowerCompradas _as_instancia_2))
  (bind _parteshidrobombacompradastodo (Variables|/Game/Instancia.Instancia_C|GetPartesHidroBombaCompradasTODO _as_instancia_2))
  (bind _textointeraccion (Variables|/Game/Interfaz/UI_PISCICOLA.UI_PISCICOLA_C|GetTextoInteraccion _refwidgetpiscicola))
  (bind _arraypiscicolas (Variables|/Game/Instancia.Instancia_C|GetArrayPiscicolas _as_instancia_3))
  (bind _indiceactual (Variables|/Game/Instancia.Instancia_C|GetIndiceActual _as_instancia_3))
  ;[1 1 1] al entrar en contacto con el trigger
  (bind _asplayer_bp (Utilities|Casting|CastToPlayerBP OtherActor))
  (Variables|/Game/BluePrints/Personaje/PlayerBP.PlayerBP_C|SetpuedeEntrarPuzzle _asplayer_bp false)
  ;;[0.8333 0.2257 0.2257] Quita la UI al salir
  (Widget|RemovefromParent (stale OnComponentBeginOverlap(Box) _returnvalue_2))
  (if (.PuzzleResuelto (Utilities|Struct|BreakPiscicolaData (Utilities|Array|Get(acopy) (Variables|/Game/Instancia.Instancia_C|GetArrayPiscicolas (Variables|Default|GetAs%20Instancia)) (stale OnComponentBeginOverlap(Box) _output_get))))
    ;[0 0 0] Widget seleccion pez
    (if (.YaSeleccionoMojarra? (Utilities|Struct|BreakPiscicolaData (Utilities|Array|Get(acopy) (Variables|/Game/Instancia.Instancia_C|GetArrayPiscicolas _as_instancia) (Variables|/Game/Instancia.Instancia_C|GetIndiceActual _as_instancia))))
      ;[1 0 0] Cambios Andres
      (if (Variables|/Game/Instancia.Instancia_C|Getdesinfectado (Variables|Default|GetAs%20Instancia))
        ;[0 0 0] Lo que se muestra dependiendo de la condicion
        (Rendering|Components|TextRender|SetText _textointeraccion "Pulse X para interactuar con la piscicola")
        (else
          (Rendering|Components|TextRender|SetText (Variables|/Game/Interfaz/UI_PISCICOLA.UI_PISCICOLA_C|GetTextoInteraccion (Variables|Default|GetRefWidGetPiscicola)) "Antes de interactuar con los peces ve a desinfectarte")))
      (else
        (bind _returnvalue_2 (UserInterface|CreateWidget "/Game/Interfaz/UI_PECES.UI_PECES_C"))
        (bind _output_get (Variables|Default|SetRefWidgetPeces _returnvalue_2))
        (UserInterface|Viewport|AddtoViewport _returnvalue_2 0)
        ;;[1 1 1] Mnaipular el mouse para seleccion
        (Variables|/Script/Engine.PlayerController|SetbShowMouseCursor _returnvalue true)
        (Input|SetInputModeUIOnly _returnvalue _output_get "DoNotLock" false)
        (bind _structout (Utilities|Struct|SetmembersinPiscicolaData (Utilities|Array|Get(acopy) _arraypiscicolas _indiceactual) true))
        (Utilities|Array|SetArrayElem _arraypiscicolas _indiceactual _structout)))
    (elif (and _partesblowercompradas _parteshidrobombacompradastodo)
      (Rendering|Components|TextRender|SetText _textointeraccion "Pulse X para construir la piscicola")
      (elif _parteshidrobombacompradastodo
        (Rendering|Components|TextRender|SetText _textointeraccion "Hacen falta comprar las partes del blower. Ve a la tienda.")
        (elif _partesblowercompradas
          (Rendering|Components|TextRender|SetText _textointeraccion "Hacen falta comprar las partes de la hidrobomba. Ve a la tienda.")
          (else
            (Rendering|Components|TextRender|SetText _textointeraccion "Hace falta comprar las partes de la hidrobomba. Ve a la tienda.")))))))

(event EventBeginPlay
  ;[1 1 1] Si el puzzle se completa cambiamos el material oscuro para ver la animacion del tranque
  (bind _asplayer_bp (Utilities|Casting|CastToPlayerBP (Game|GetPlayerCharacter 0)))
  (Variables|Default|SetAs%20Player%20BP _asplayer_bp)
  (bind _asinstancia (Utilities|Casting|CastToInstancia (Game|GetGameInstance)))
  (bind _output_get (Variables|Default|SetAs%20Instancia _asinstancia))
  (if (.PuzzleResuelto (Utilities|Struct|BreakPiscicolaData (Utilities|Array|Get(acopy) (Variables|/Game/Instancia.Instancia_C|GetArrayPiscicolas _output_get) (Variables|Default|GetIndicePiscicola))))
    (Sprite|SetFlipbook (Variables|Default|GetTanque) "/Game/Assets/Exterior/Flipbooks/Tanques/Tanque.Tanque")))

(fn ConstructionScript)