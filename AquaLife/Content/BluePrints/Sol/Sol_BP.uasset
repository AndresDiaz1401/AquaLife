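; Sun light Blueprint that runs the day/night cycle and the game's 12-hour AM/PM clock and day counter.
; BeginPlay restores hour, AM/PM and day from the Instancia GameInstance, carrying time across levels.
; Each Tick, DefinirFranja maps hour and AM/PM to a stepped light intensity.
; Roughly every seven seconds the hour advances and saves back, flipping AM/PM after 12 and incrementing the day on switching to PM.
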(event EventBeginPlay
  ;[1 1 1] Comenzar desde los ultimos datos guardados en el anterior nivel
  (bind _asinstancia (Utilities|Casting|CastToInstancia (Game|GetGameInstance)))
  (Variables|Default|SetHoraDia (Variables|/Game/Instancia.Instancia_C|GetHoraDiaGuardar _asinstancia))
  (Variables|Default|Setam/pm (Variables|/Game/Instancia.Instancia_C|Getam/pmGuardar _asinstancia))
  (Variables|Default|SetDias (Variables|/Game/Instancia.Instancia_C|GetDiaGuardar _asinstancia)))

(event EventTick
  (params (DeltaSeconds :type Float%20%28single-precision%29))
  (bind _returnvalue (Utilities|Time|GetGameTimeinSeconds))
  ;[1 1 1] Ciclo dia y noche
  ;;[1 1 1] Intensidad de la luz
  (Utilities|FlowControl|Sequence
    (:then_0
      (CallFunction|DefinirFranja)
      (Rendering|Components|Light|SetIntensity (Variables|Default|GetLightComponent) (Variables|Default|Getintensidad))
      ;;[1 1 1] Pasar horas
      (Variables|Default|SettiempoFinal _returnvalue)
      (bind _output_get (Variables|Default|SetreiniciarTiempo (> (- (Variables|Default|GettiempoFinal) (Variables|Default|GettiempoInicial)) 7.0)))
      (if _output_get
        (Variables|Default|SettiempoInicial _returnvalue)
        (bind _asinstancia (Utilities|Casting|CastToInstancia (Game|GetGameInstance)))
        (Variables|/Game/Instancia.Instancia_C|SetHoraDiaGuardar _asinstancia (+ (Variables|Default|GetHoraDia) 1))
        (Variables|Default|SetHoraDia (+ (Variables|Default|GetHoraDia) 1))
        (Variables|Default|SetCambioHora true)
        (if (Variables|Default|Getam/pm)
          _
          (else
            _))
        (if (> (Variables|Default|GetHoraDia) 12)
          (Variables|Default|SetHoraDia 1)
          (if (>= (Variables|/Game/Instancia.Instancia_C|GetHoraDiaGuardar _asinstancia) 12)
            (Variables|/Game/Instancia.Instancia_C|SetHoraDiaGuardar _asinstancia 1)
            (bind _output_get_2 (Variables|Default|Setam/pm (not (Variables|Default|Getam/pm))))
            (Variables|/Game/Instancia.Instancia_C|Setam/pmGuardar _asinstancia _output_get_2)
            (if _output_get_2
              (bind _output_get_3 (Variables|Default|SetDias (+ (Variables|Default|GetDias) 1)))
              (Variables|/Game/Instancia.Instancia_C|SetDiaGuardar _asinstancia _output_get_3))))))))

(fn ConstructionScript)

(fn DefinirFranja
  ;[1 1 1] Establecer iluminosidad AM/PM
  (if (Variables|Default|Getam/pm)
    (Variables|Default|SetFranja "PM")
    ;[1 1 1] Iluminosidad PM
    (switch int (Variables|Default|GetHoraDia)
      (:0
        (Variables|Default|Setintensidad 2.5))
      (:1
        (Variables|Default|Setintensidad 2.5))
      (:2
        (Variables|Default|Setintensidad 2.5))
      (:3
        (Variables|Default|Setintensidad 2.5))
      (:4
        (Variables|Default|Setintensidad 1.5))
      (:5
        (Variables|Default|Setintensidad 1.0))
      (:6
        (Variables|Default|Setintensidad 0.5))
      (:7
        (Variables|Default|Setintensidad 0.3))
      (:8
        (Variables|Default|Setintensidad 0.3))
      (:9
        (Variables|Default|Setintensidad 0.1))
      (:10
        (Variables|Default|Setintensidad 0.1))
      (:11
        (Variables|Default|Setintensidad 0.1))
      (:12
        (Variables|Default|Setintensidad 0.1)))
    (else
      (Variables|Default|SetFranja "AM")
      ;[1 1 1] Iluminosidad AM
      (switch int (Variables|Default|GetHoraDia)
        (:0
          (Variables|Default|Setintensidad 0.1))
        (:1
          (Variables|Default|Setintensidad 0.1))
        (:2
          (Variables|Default|Setintensidad 0.1))
        (:3
          (Variables|Default|Setintensidad 0.1))
        (:4
          (Variables|Default|Setintensidad 0.1))
        (:5
          (Variables|Default|Setintensidad 1.0))
        (:6
          (Variables|Default|Setintensidad 1.5))
        (:7
          (Variables|Default|Setintensidad 2.0))
        (:8
          (Variables|Default|Setintensidad 2.5))
        (:9
          (Variables|Default|Setintensidad 2.5))
        (:10
          (Variables|Default|Setintensidad 2.5))))))

(fn ContadorHora
  (Variables|Default|SetHoraDia 0))