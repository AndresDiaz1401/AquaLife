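; BacteriaBP is a patrolling enemy bacterium with a Paper2D flipbook that can hurt the player and be killed.
; Tick moves it along X, flipping direction and sprite from the Choco flag, which is not set here, until Tiempomuerte is true.
; Sphere overlap takes one Vida from PlayerBP or, for JabonazoBP attacks, sets Tiempomuerte and kills it.
; Box overlap with the player also kills it; both deaths play animation and sound before destroying the actor.
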(event OnComponentBeginOverlap(Sphere)
  (params (OverlappedComponent :type Primitive%20Component%20Object%20Reference) (OtherActor :type Actor%20Object%20Reference) (OtherComp :type Primitive%20Component%20Object%20Reference) (OtherBodyIndex :type Integer) (bFromSweep :type Boolean) (SweepResult :type Hit%20Result%20Structure%20%28by%20ref%29))
  (bind _paperflipbook (Variables|Default|GetPaperFlipbook))
  ;[1 1 1] Si entra en contacto con el ataque
  (CallFunction|RestarVida OtherActor)
  (Utilities|Casting|CastToJabonazoBP OtherActor)
  ;;[1 1 1] Activa la animacion de muerte y sonido
  (Sprite|SetFlipbook _paperflipbook "/Game/BluePrints/Bacteria/FlipBooksBacteria/MuerteBacteria.MuerteBacteria")
  (Variables|Default|Settiempomuerte true)
  (Audio|PlaySound2D "/Game/sonidos/slimeMuerte.slimeMuerte" 1.0 1.0 0.0 0 0)
  ;;[1 1 1] Esperar a que se acabe la animacion y destruye el actor
  (Utilities|FlowControl|Delay (Class|PaperFlipbookComponent|GetFlipbookLength _paperflipbook))
  (Actor|DestroyActor))

(event OnComponentBeginOverlap(Box)
  (params (OverlappedComponent :type Primitive%20Component%20Object%20Reference) (OtherActor :type Actor%20Object%20Reference) (OtherComp :type Primitive%20Component%20Object%20Reference) (OtherBodyIndex :type Integer) (bFromSweep :type Boolean) (SweepResult :type Hit%20Result%20Structure%20%28by%20ref%29))
  (bind _paperflipbook (Variables|Default|GetPaperFlipbook))
  ;[1 1 1] Si entra en contacto con el jugador
  (Utilities|Casting|CastToPlayerBP OtherActor)
  ;;[1 1 1] Animacion y sonido muerte
  (Sprite|SetFlipbook _paperflipbook "/Game/BluePrints/Bacteria/FlipBooksBacteria/MuerteBacteria.MuerteBacteria")
  (Audio|PlaySound2D "/Game/sonidos/slimeMuerte.slimeMuerte" 1.0 1.0 0.0 0 0)
  ;;[1 1 1] Espera a que se acabe la animacion y destruye el actor
  (Utilities|FlowControl|Delay (Class|PaperFlipbookComponent|GetFlipbookLength _paperflipbook))
  (Actor|DestroyActor))

(event EventBeginPlay)

(event Collision|EventActorBeginOverlap
  (params (OtherActor :type Actor%20Object%20Reference)))

(event EventTick
  (params (DeltaSeconds :type Float%20%28single-precision%29))
  (bind _returnvalue (Transformation|GetActorLocation))
  (bind _paperflipbook (Variables|Default|GetPaperFlipbook))
  ;[1 1 1] Movimiento de la bacteria
  (Transformation|SetActorLocation (Math|Vector|MakeVector (+ (* DeltaSeconds (Variables|Default|Getvelocidad) (Variables|Default|Getdireccion)) (.x _returnvalue)) (.y _returnvalue) (.z _returnvalue)) false false)
  (if (not (Variables|Default|Gettiempomuerte))
    ;[1 1 1] Si choco con una pared cambia de direccion
    (if (Variables|Default|Getchoco)
      (Variables|Default|Setdireccion -1.0)
      (Transformation|SetRelativeScale3D _paperflipbook "-1.000000,1.000000,1.000000")
      (else
        (Variables|Default|Setdireccion 1.0)
        (Transformation|SetRelativeScale3D _paperflipbook "1.000000,1.000000,1.000000")))))

(fn ConstructionScript)

(fn RestarVida
  (params (Object :type Object%20Object%20Reference))
  (bind _asplayer_bp (Utilities|Casting|CastToPlayerBP Object))
  (Variables|/Game/BluePrints/Personaje/PlayerBP.PlayerBP_C|Setvida _asplayer_bp (- (Variables|/Game/BluePrints/Personaje/PlayerBP.PlayerBP_C|Getvida _asplayer_bp) 1))
  (Audio|PlaySound2D "/Game/sonidos/daño.daño" 1.0 1.0 0.0 0 0))