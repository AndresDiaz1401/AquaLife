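; Player character with a sprite that switches between four-direction movement and side-scrolling platformer via the game instance's Plataforma flag.
; Enhanced Input drives movement, jump and click state; platformer mode rotates the spring arm, drops vertical movement, tracks jumping on Tick and enables delayed, direction-based JabonazoBP attacks with sound.
; Pressing X saves player position, then opens the fish or puzzle-info level depending on puzzle and purchased-part progress.
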(event Input|EnhancedActionEvents|EnhancedInputActionMouseClick
  (params (ActionValue :type Boolean) (ElapsedSeconds :type Float%20%28double-precision%29) (TriggeredSeconds :type Float%20%28double-precision%29) (InputAction :type Input%20Action%20Object%20Reference :default "/Game/EntradasAccion/MouseClick.MouseClick"))
  ;[1 1 1] Detectar cuando el jugador hace click para el puzzle
  (:Triggered
    (Variables|Default|SetIsClicked true))
  (:Completed
    (Variables|Default|SetIsClicked false)))

(event Input|EnhancedActionEvents|EnhancedInputActionplayerMove
  (params (ActionValue :type Vector%202D%20Structure) (ElapsedSeconds :type Float%20%28double-precision%29) (TriggeredSeconds :type Float%20%28double-precision%29) (InputAction :type Input%20Action%20Object%20Reference :default "/Game/EntradasAccion/playerMove.playerMove"))
  ;[1 1 1] Movimoento personaje
  (:Triggered
    (Pawn|Input|AddMovementInput "1.000000,0.000000,0.000000" (.x ActionValue) false)
    ;;[1 1 1] Si es plataforma, ajusta el movimiento del personaje
    (if (Variables|/Game/Instancia.Instancia_C|GetPlataforma (Variables|Default|GetAs%20Instancia))
      (Variables|Default|Setdireccion (Math|Vector2D|MakeVector2D (.x ActionValue) 0.0))
      (else
        (Pawn|Input|AddMovementInput "0.000000,-1.000000,0.000000" (.y ActionValue) false)
        (Variables|Default|Setdireccion (Math|Vector2D|MakeVector2D (.x ActionValue) (.y ActionValue))))))
  (:Started
    (Variables|Default|Setmoviendo true))
  (:Completed
    (Variables|Default|Setmoviendo false)))

(event Input|EnhancedActionEvents|EnhancedInputActionplayerJump
  (params (ActionValue :type Boolean) (ElapsedSeconds :type Float%20%28double-precision%29) (TriggeredSeconds :type Float%20%28double-precision%29) (InputAction :type Input%20Action%20Object%20Reference :default "/Game/EntradasAccion/playerJump.playerJump"))
  ;[1 1 1] Funcion saltar
  (Character|Jump))

(event Input|EnhancedActionEvents|EnhancedInputActionPlayerAttack
  (params (ActionValue :type Vector%202D%20Structure) (ElapsedSeconds :type Float%20%28double-precision%29) (TriggeredSeconds :type Float%20%28double-precision%29) (InputAction :type Input%20Action%20Object%20Reference :default "/Game/EntradasAccion/PlayerAttack.PlayerAttack"))
  ;[1 1 1] El jugador ataca
  (:Started
    (if (Variables|/Game/Instancia.Instancia_C|GetPlataforma (Variables|Default|GetAs%20Instancia))
      (Variables|Plataforma|Setatacando true)
      ;;[1 1 1] Deteta direccion del ataque
      (if (>= (.X (Math|Vector2D|BreakVector2D (Variables|Default|Getdireccion))) 0.0)
        ;;[1 1 1] Aparece el ataque y suena
        (Utilities|FlowControl|Delay 0.5)
        (Game|SpawnActorfromClass "/Game/BluePrints/Personaje/JabonazoBP.JabonazoBP_C" (Transformation|GetWorldTransform (Variables|Default|GetJabonazoDerecha)) "Undefined" "MultiplyWithRoot" 0 0)
        (Audio|PlaySound2D 0 1.0 1.0 0.0 0 0)
        (else
          ;;[1 1 1] Aparece el ataque y suena
          (Utilities|FlowControl|Delay 0.5)
          (Game|SpawnActorfromClass "/Game/BluePrints/Personaje/JabonazoBP.JabonazoBP_C" (Transformation|GetWorldTransform (Variables|Default|GetJabonazoIzquierda)) "Undefined" "MultiplyWithRoot" 0 0)
          (Audio|PlaySound2D 0 1.0 1.0 0.0 0 0)))))
  (:Completed
    (Utilities|FlowControl|Delay 0.5)
    (Variables|Plataforma|Setatacando false)))

(event EventBeginPlay
  ;[1 1 1] Asociar al jugador con la entrada de acciones
  (bind _asplayer_controller (Utilities|Casting|CastToPlayerController (Pawn|GetController)))
  (bind _asinstancia (Utilities|Casting|CastToInstancia (Game|GetGameInstance)))
  (Variables|Default|SetAs%20Instancia _asinstancia)
  (Input|AddMappingContext (PlayerController|LocalPlayerSubsystems|GetEnhancedInputLocalPlayerSubsystem _asplayer_controller) "/Game/EntradasAccion/InputPLayer.InputPLayer" 0 "(bIgnoreAllPressedKeysUntilRelease=True,bForceImmediately=False,bNotifyUserSettings=False)")
  ;;[1 1 1] Si el nivel es una plataforma rota al jugador
  (if (Variables|/Game/Instancia.Instancia_C|GetPlataforma (Variables|Default|GetAs%20Instancia))
    (Transformation|SetWorldRotation (Variables|Default|GetSpringArm) "0.000000,-90.000000,0.000000" false false)
    (Transformation|SetWorldRotation (Variables|Default|GetSprite) "0, 0, 0" false false)))

(event Collision|EventActorBeginOverlap
  (params (OtherActor :type Actor%20Object%20Reference)))

(event EventTick
  (params (DeltaSeconds :type Float%20%28single-precision%29))
  ;[1 1 1] El juego es plataformero?
  (if (Variables|/Game/Instancia.Instancia_C|GetPlataforma (Variables|Default|GetAs%20Instancia))
    ;[1 1 1] Si es plataforma activa salto
    (if (AI|Components|NavMovement|IsMovingonGround (Variables|Character|GetCharacterMovement))
      (Variables|Plataforma|Setsaltando false)
      (else
        (Variables|Plataforma|Setsaltando true)))))

(event Input|KeyboardEvents|X
  (params (Key :type Key%20Structure :default "None"))
  (bind _as_instancia (Variables|Default|GetAs%20Instancia))
  (bind _as_instancia_2 (Variables|Default|GetAs%20Instancia))
  ;[1 1 1] presiona x para entrar al puzzle
  (:Pressed
    ;;[0 0 0] al dar x tambien se guarda la posicion
    (bind _returnvalue (SaveGame|CreateSaveGameObject "/Game/GuadarCosas.GuadarCosas_C"))
    (Variables|/Game/GuadarCosas.GuadarCosas_C|SetPosicionJugador _returnvalue (Transformation|GetActorLocation))
    (SaveGame|SaveGametoSlot _returnvalue "1")
    (Development|PrintString "guardo posicion")
    (if (.PuzzleResuelto (Utilities|Struct|BreakPiscicolaData (Utilities|Array|Get(acopy) (Variables|/Game/Instancia.Instancia_C|GetArrayPiscicolas _as_instancia) (Variables|/Game/Instancia.Instancia_C|GetIndiceActual _as_instancia))))
      (Game|OpenLevel(byName) "LevelPeces")
      (elif (and (Variables|/Game/Instancia.Instancia_C|GetPartesHidroBombaCompradasTODO _as_instancia_2) (Variables|/Game/Instancia.Instancia_C|GetPartesBlowerCompradas _as_instancia_2))
        (Game|OpenLevel(byName) "LvlVacioInfoPuzzle")))))

(fn ConstructionScript)