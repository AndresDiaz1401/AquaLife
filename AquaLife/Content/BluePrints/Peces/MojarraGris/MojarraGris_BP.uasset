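; MojarraGris_BP is a grey mojarra fish that swims horizontally along the world X axis.
; BeginPlay caches the Instancia game instance and, if that cast succeeds, sets DirMoveGris to true.
; Tick records X velocity in DireccionGris and applies movement input toward positive or negative X according to DirMoveGris.
; Nothing in this graph flips the direction or reads the cached instance.
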(event EventBeginPlay
  ;[1 1 1] Movimiento del pez
  (bind _asinstancia (Utilities|Casting|CastToInstancia (Game|GetGameInstance)))
  (Variables|Default|SetAs%20Instancia _asinstancia)
  (Variables|Default|SetdirMoveGris true))

(event Collision|EventActorBeginOverlap
  (params (OtherActor :type Actor%20Object%20Reference)))

(event EventTick
  (params (DeltaSeconds :type Float%20%28single-precision%29))
  ;[1 1 1] Movimiento del pez
  (Variables|Default|SetdireccionGris (.x (Transformation|GetVelocity)))
  (if (Variables|Default|GetdirMoveGris)
    (Pawn|Input|AddMovementInput "1.000000,0.000000,0.000000" 1.0 false)
    (else
      (Pawn|Input|AddMovementInput "-1.000000,0.000000,0.000000" 1.0 false))))

(fn ConstructionScript)