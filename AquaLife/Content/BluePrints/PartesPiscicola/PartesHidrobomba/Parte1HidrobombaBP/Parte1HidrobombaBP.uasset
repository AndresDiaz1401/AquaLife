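; Draggable first piece of the Hidrobomba assembly puzzle, moved with the mouse and color-coded by flipbook.
; Tick compares the deprojected cursor to the sprite within an X/Y tolerance and reads click state from the Instancia GameInstance.
; Its shared SeleccionPieza flag limits grabbing to one piece; Mover keeps the capsule following the cursor.
; The piece shows yellow when dragged, red when released, and locks green once ParteCorrecta is set outside this graph.
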(event EventBeginPlay
  ;[1 1 1] Referenciar la instancia
  (bind _asinstancia (Utilities|Casting|CastToInstancia (Game|GetGameInstance)))
  (Variables|Default|SetAs%20Instancia _asinstancia))

(event EventTick
  (params (DeltaSeconds :type Float%20%28single-precision%29))
  (bind _returnvalue (Game|GetPlayerController 0))
  (bind _returnvalue_2 (Game|GetPlayerController 0))
  (bind _as_instancia (Variables|Default|GetAs%20Instancia))
  (bind _sprite (Variables|Default|GetSprite))
  (bind _worldlocation (Game|Player|ConvertMouseLocationToWorldSpace _returnvalue))
  (bind _returnvalue_3 (Transformation|GetWorldLocation _sprite))
  (bind _worldlocation_2 (Game|Player|ConvertMouseLocationToWorldSpace _returnvalue_2))
  ;[0 0 0] Movimiento de las piezas y cambio de color solo usamdo el "Set FlipBook"
  ;;[1 1 1] Si la pieza esta en su lugar corecto colo==verde
  (if (Variables|Default|GetParte%20Correcta)
    (Sprite|SetFlipbook (Variables|Default|GetSprite) "/Game/Assets/piezasPiscicolas/PartesHidrobomba/PartesVerdesHidrobomba/flipbook/Parte_1_verde_Hidrobomba.Parte_1_verde_Hidrobomba")
    (elif (and (<= (Math|Float|Absolute(Float) (- (.x _worldlocation) (.x _returnvalue_3))) 2e+01) (<= (Math|Float|Absolute(Float) (- (.y _worldlocation) (.y _returnvalue_3))) 1e+01))
      (if (Variables|/Game/Instancia.Instancia_C|GethaciendoClick (Variables|Default|GetAs%20Instancia))
        (if (Variables|/Game/Instancia.Instancia_C|GetseleccionPieza _as_instancia)
          (Variables|/Game/Instancia.Instancia_C|SetseleccionPieza _as_instancia false)
          (Variables|Default|Setmover true)
          ;;[1 1 1] Cambiar el color==Verde , si la posicion corresponde a la capsula de la parte seleccionada "en este caso parte1"
          (Transformation|SetWorldLocation (Variables|Default|GetCapsuleComponent) (Math|Vector|MakeVector (.x _worldlocation_2) (.y _worldlocation_2) 0.0) false false :!label _label)
          (Sprite|SetFlipbook (Variables|Default|GetSprite) "/Game/Assets/piezasPiscicolas/PartesHidrobomba/PartesAmarillasHidrobomba/flipbook/Parte_1_amarillo_Hidrobomba.Parte_1_amarillo_Hidrobomba"))
        (else
          ;;[1 1 1] Si la pieza esta en su lugar corecto colo==rojo
          (Variables|/Game/Instancia.Instancia_C|SetseleccionPieza _as_instancia true)
          (Variables|Default|Setmover false)
          (Sprite|SetFlipbook (Variables|Default|GetSprite) "/Game/Assets/piezasPiscicolas/PartesHidrobomba/PartesRojasHidrobomba/flipbook/Parte_1_rojo_Hidrobomba.Parte_1_rojo_Hidrobomba")))
      (elif (Variables|Default|GetMover)
        (goto _label)))))

(fn ConstructionScript)